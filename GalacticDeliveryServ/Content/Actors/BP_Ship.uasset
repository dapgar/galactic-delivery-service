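; Player-flown ship pawn with a state machine: on land, takeoff, flying and landing.
; Movement input on land triggers a timeline takeoff; in flight it drives FloatingPawnMovement, alongside forward thrust from a curve of camera turn rate.
; The hull eases toward control rotation and tilts with input.
; At low speed, a downward box trace finds ground and starts a timeline landing that lowers and levels the ship.
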(event `self.ReceiveTick`
  (params (DeltaSeconds :type "Float (single-precision)"))
  (bind _returnvalue (`self.GetControlRotation`))
  (bind _returnvalue_2 (`self.K2_GetActorLocation`))
  (bind _shipcolliderbox (`self.ShipColliderBox`))
  (bind _shipcomponents (`self.ShipComponents`))
  (bind _returnvalue_3 (`PawnMovementComponent.GetLastInputVector` (`self.FloatingPawnMovement`)))
  (bind (_relativerotation_roll _relativerotation_pitch) (`KismetMathLibrary.BreakRotator` (`SceneComponent.RelativeRotation` _shipcomponents)))
  (switch `/Game/E_ShipStates` (`self.State`)
    (:`NewEnumerator2`
      (`|ExecutionSequence`
        (:`then_0`
          (bind _output_get (set `self.PreviousMousePos` (`self.CurrentMousePos`)))
          (bind _output_get_2 (set `self.CurrentMousePos` (`KismetMathLibrary.Conv_RotatorToVector` (`self.GetControlRotation`))))
          (bind _output_get_3 (set `self.MouseMovementMagnitude` (* (`KismetMathLibrary.VSize` (- _output_get_2 _output_get)) 10.0)))
          (bind _returnvalue_4 (`CurveFloat.GetFloatValue` (`self.MouseDeltaDecelerationCurve`) _output_get_3))
          (`self.AddMovementInput` (`KismetMathLibrary.GetForwardVector` (`self.GetControlRotation`)) _returnvalue_4)
          (`KismetSystemLibrary.PrintString` (`KismetStringLibrary.Conv_DoubleToString` _returnvalue_4))
          (`KismetSystemLibrary.PrintString` (`KismetStringLibrary.Conv_DoubleToString` (`KismetMathLibrary.VSize` (`self.GetVelocity`)))))
        (:`then_1`
          ;[1 1 1] Rotate Ship to follow mouse
          (bind _output_get_4 (set `self.CurrentShipRotation` (`KismetMathLibrary.RInterpTo` (`self.CurrentShipRotation`) (`self.GetControlRotation`) DeltaSeconds (`self.ShipInterpSpeed`))))
          (`SceneComponent.K2_SetWorldRotation` (`self.ShipRotationPoint`) _output_get_4 false false)
          ;[1 1 1] Rotates the ship to tilt while moving
          (`SceneComponent.K2_SetRelativeRotation` _shipcomponents (`KismetMathLibrary.MakeRotator` (`KismetMathLibrary.FInterpTo` _relativerotation_roll (* (`KismetMathLibrary.Dot_VectorVector` _returnvalue_3 (`KismetMathLibrary.GetRightVector` _returnvalue)) (`self.ShipTiltAmount`)) DeltaSeconds (`self.ShipTiltInerp`)) (`KismetMathLibrary.FInterpTo` _relativerotation_pitch (* (`KismetMathLibrary.Dot_VectorVector` _returnvalue_3 (`KismetMathLibrary.GetForwardVector` _returnvalue)) (* (`self.ShipTiltAmount`) -1.0)) DeltaSeconds (`self.ShipTiltInerp`))) false false))
        (:`then_2`
          (if (< (`KismetMathLibrary.VSize` (`self.GetVelocity`)) (`self.MaxSpeedForLanding`))
            ;[1 1 1] Check if we can Land
            (bind (_outhit _returnvalue_5) (`KismetSystemLibrary.BoxTraceSingle` :`Start` _returnvalue_2 :`End` (- _returnvalue_2 (`KismetMathLibrary.MakeVector` 0.0 0.0 (`self.MinHeighToLand`))) :`HalfSize` (`BoxComponent.GetScaledBoxExtent` _shipcolliderbox) :`Orientation` (`KismetMathLibrary.Conv_VectorToRotator` (`SceneComponent.GetForwardVector` _shipcolliderbox)) :`TraceChannel` "TraceTypeQuery1" :`DrawDebugType` "ForOneFrame"))
            (if _returnvalue_5
              (set `self.EndTakeOffPosition` (`.Location` (`GameplayStatics.BreakHitResult` _outhit)))
              (`self.StartLanding`))))))))

(event `self.ReceiveBeginPlay`)

(event `Takeoff`
  ;[1 1 1] Handles the takeoff sequence of the ship
  ;;[0 0.05098 1] Prepare ship for takeoff
  (`self.HandleShipStateChange` "NewEnumerator4")
  (set `self.StartTakeOffPosition` (`self.K2_GetActorLocation`))
  (set `self.EndTakeOffPosition` (+ (`self.StartTakeOffPosition`) (`KismetMathLibrary.MakeVector` 0.0 0.0 (`self.ZIncreaseTakeOff`))))
  (`TimelineComponent.SetPlayRate` (`self.T_Takeoff`) 0.8)
  ;;[0 0.05098 1] Moves the ship up/down to preform manuver
  (bind (_direction _verticalmovementalpha) (`Timeline|T_Takeoff` :!via `PlayFromStart`)
    (:`Update`
      (`self.K2_SetActorLocation` (`KismetMathLibrary.VLerp` (`self.StartTakeOffPosition`) (`self.EndTakeOffPosition`) _verticalmovementalpha) true))
    (:`Finished`
      (`self.HandleShipStateChange` "NewEnumerator2"))))

(event `StartLanding`
  ;[1 1 1] Handles the takeoff sequence of the ship
  ;;[0 0.05098 1] Prepare for landing
  (`self.HandleShipStateChange` "NewEnumerator3")
  (set `self.StartTakeOffPosition` (`self.K2_GetActorLocation`))
  (set `self.StartShipLandRotation` (`SceneComponent.K2_GetComponentRotation` (`self.ShipRotationPoint`)))
  (set `self.StartLandRelativeRotation` (`SceneComponent.RelativeRotation` (`self.ShipComponents`)))
  (`TimelineComponent.SetPlayRate` (`self.T_Land`) 1.0)
  ;;[0 0.05098 1] Moves and rotates ship to landing position
  (bind (_direction _verticalmovementalpha _shiprotationalpha) (`Timeline|T_Land` :!via `PlayFromStart`)
    (:`Update`
      (`self.K2_SetActorLocation` (`KismetMathLibrary.VLerp` (`self.StartTakeOffPosition`) (`self.EndTakeOffPosition`) _verticalmovementalpha) true)
      (`SceneComponent.K2_SetWorldRotation` (`self.ShipRotationPoint`) (`KismetMathLibrary.RLerp` (`self.StartShipLandRotation`) (`KismetMathLibrary.Conv_VectorToRotator` (`SceneComponent.GetForwardVector` (`self.ShipColliderBox`))) _shiprotationalpha) false false)
      (`SceneComponent.K2_SetRelativeRotation` (`self.ShipComponents`) (`KismetMathLibrary.RLerp` (`self.StartLandRelativeRotation`) (struct) _shiprotationalpha) false false))
    (:`Finished`
      (`self.HandleShipStateChange` "NewEnumerator1"))))

(event `InputAxis|LookUp`
  (params (AxisValue :type "Float (single-precision)"))
  ;[1 1 1] Handle Input
  ;;[0 0.05186 1] Rotates Camera
  (`self.AddControllerPitchInput` AxisValue))

(event `InputAxis|MoveForward`
  (params (AxisValue :type "Float (single-precision)"))
  ;[1 1 1] Handle Input
  ;;[0 0.05098 1] Moves Ship
  (switch `/Game/E_ShipStates` (`self.State`)
    (:`NewEnumerator1`
      (if (!= AxisValue 0.0)
        (`self.Takeoff`)))
    (:`NewEnumerator2`
      (`self.AddMovementInput` (`KismetMathLibrary.GetForwardVector` (`self.GetControlRotation`)) AxisValue))))

(event `InputAxis|LookRight`
  (params (AxisValue :type "Float (single-precision)"))
  ;[1 1 1] Handle Input
  ;;[0 0.05186 1] Rotates Camera
  (`self.AddControllerYawInput` AxisValue))

(event `InputAxis|MoveRight`
  (params (AxisValue :type "Float (single-precision)"))
  ;[1 1 1] Handle Input
  ;;[0 0.05098 1] Moves Ship
  (switch `/Game/E_ShipStates` (`self.State`)
    (:`NewEnumerator1`
      (if (!= AxisValue 0.0)
        (`self.Takeoff`)))
    (:`NewEnumerator2`
      (`self.AddMovementInput` (`KismetMathLibrary.GetRightVector` (`self.GetControlRotation`)) AxisValue))))

(event `self.ReceivePossessed`
  (params (NewController :type "Controller Object Reference"))
  (set `self.CurrentShipRotation` (`SceneComponent.K2_GetComponentRotation` (`self.ShipRotationPoint`))))

(event `InputAxis|MoveUp`
  (params (AxisValue :type "Float (single-precision)"))
  ;[1 1 1] Handle Input
  ;;[0 0.05098 1] Moves Ship
  (switch `/Game/E_ShipStates` (`self.State`)
    (:`NewEnumerator1`
      (if (!= AxisValue 0.0)
        (`self.Takeoff`)))
    (:`NewEnumerator2`
      (`self.AddMovementInput` (`KismetMathLibrary.GetUpVector` (`self.GetControlRotation`)) AxisValue))))

(fn `HandleShipStateChange`
  (params (`New State` :type "/Game/E_ShipStates Enum" :default "NewEnumerator0"))
  (bind _output_get (set `self.State` `New State`))
  (switch `/Game/E_ShipStates` _output_get
    (:`NewEnumerator1`
      (set `self.bUseControllerRotationYaw` false :!label _label))
    (:`NewEnumerator4`
      (goto _label))
    (:`NewEnumerator2`
      (set `self.bUseControllerRotationYaw` true))
    (:`NewEnumerator3`
      (goto _label))))

(fn `UserConstructionScript`)